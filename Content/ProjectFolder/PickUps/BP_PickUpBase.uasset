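; Base pickup actor that tells players when they enter or leave its pickup range.
; On the server only, begin and end overlaps on PickUpBox send OverlapPickUpMessage through INT_Player, passing the pickup and an overlap flag.
; GetHealthAmount returns zero here, and the pickup itself applies no effect.
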(event OnComponentBeginOverlap(PickUpBox)
  (params (OverlappedComponent :type Primitive%20Component%20Object%20Reference) (OtherActor :type Actor%20Object%20Reference) (OtherComp :type Primitive%20Component%20Object%20Reference) (OtherBodyIndex :type Integer) (bFromSweep :type Boolean) (SweepResult :type Hit%20Result%20Structure%20%28by%20ref%29))
  (if (Networking|IsServer)
    (if (Utilities|DoesObjectImplementInterface OtherActor "/Game/ProjectFolder/Character/Interfaces/INT_Player.INT_Player_C")
      (Class|INTPlayer|OverlapPickUp(Message) OtherActor self true))))

(event OnComponentEndOverlap(PickUpBox)
  (params (OverlappedComponent :type Primitive%20Component%20Object%20Reference) (OtherActor :type Actor%20Object%20Reference) (OtherComp :type Primitive%20Component%20Object%20Reference) (OtherBodyIndex :type Integer))
  (if (Networking|IsServer)
    (if (Utilities|DoesObjectImplementInterface OtherActor "/Game/ProjectFolder/Character/Interfaces/INT_Player.INT_Player_C")
      (Class|INTPlayer|OverlapPickUp(Message) OtherActor self false))))

(event EventBeginPlay)

(event Collision|EventActorBeginOverlap
  (params (OtherActor :type Actor%20Object%20Reference)))

(event EventTick
  (params (DeltaSeconds :type Float%20%28single-precision%29)))

(fn ConstructionScript)

(fn GetHealthAmount
  (return 0.0))